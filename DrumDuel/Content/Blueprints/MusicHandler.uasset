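; Music handler that selects a jazz, rock or funk soundtrack and plays the track for the current round phase.
; On BeginPlay it casts the game instance to GameMode and uses SongChoice and GameMode to assign opener, between, end and three round sections, with jazz as default and alternate, mostly AI-named, tracks for mode 1.
; MusicCalled reads the first Beat actor's Phase and plays the matching section once, via DoOnce.
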(event Custom|Music%20Called
  (bind _outactors (Actor|GetAllActorsOfClass "/Game/Blueprints/Beat.Beat_C"))
  (switch int (Variables|/Game/Blueprints/Beat.Beat_C|GetPhase (Utilities|Array|Get(acopy) _outactors))
    (:1
      (Utilities|FlowControl|DoOnce false
        (:Completed
          (Audio|Components|Audio|Play (Variables|Default|GetSection1) 0.0))))
    (:2
      (Utilities|FlowControl|DoOnce false
        (:Completed
          (Audio|Components|Audio|Play (Variables|Default|GetSection2) 0.0))))
    (:3
      (Utilities|FlowControl|DoOnce false
        (:Completed
          (Audio|Components|Audio|Play (Variables|Default|GetSection3) 0.0))))))

(event EventBeginPlay
  (bind _asgame_mode (Utilities|Casting|CastToGameMode (Game|GetGameInstance)))
  (switch int (Variables|/Game/Blueprints/GameMode.GameMode_C|GetSongChoice _asgame_mode)
    (:Default
      (Variables|Default|SetSectionOpener (Variables|Default|GetJazzOpen_Cue) :!label _label)
      (Variables|Default|SetSectionBetween (Variables|Default|GetJazzBetween_Cue))
      (Variables|Default|SetSectionEnd (Variables|Default|GetJazzEnd))
      (switch int (Variables|/Game/Blueprints/GameMode.GameMode_C|GetGameMode _asgame_mode)
        (:Default
          (Variables|Default|SetSection1 (Variables|Default|GetJazzRound1_OG_) :!label _label_2)
          (Variables|Default|SetSection2 (Variables|Default|GetJazzRound2))
          (Variables|Default|SetSection3 (Variables|Default|GetJazzRound3)))
        (:0
          (goto _label_2))
        (:1
          (Variables|Default|SetSection1 (Variables|Default|GetAIJazzRound1))
          (Variables|Default|SetSection2 (Variables|Default|GetAIJazzRound2))
          (Variables|Default|SetSection3 (Variables|Default|GetAIJazzRound3)))))
    (:1
      (goto _label))
    (:2
      (Variables|Default|SetSectionOpener (Variables|Default|GetRockOpen_Cue))
      (Variables|Default|SetSectionBetween (Variables|Default|GetRockBetween_Cue))
      (Variables|Default|SetSectionEnd (Variables|Default|GetRockEnd))
      (switch int (Variables|/Game/Blueprints/GameMode.GameMode_C|GetGameMode _asgame_mode)
        (:0
          (Variables|Default|SetSection1 (Variables|Default|GetRockRound1_OG_))
          (Variables|Default|SetSection2 (Variables|Default|GetRockRound2))
          (Variables|Default|SetSection3 (Variables|Default|GetRockRound3)))
        (:1
          (Variables|Default|SetSection1 (Variables|Default|GetRockRound1))
          (Variables|Default|SetSection2 (Variables|Default|GetAIRockRound2))
          (Variables|Default|SetSection3 (Variables|Default|GetAIRockRound3)))))
    (:3
      (Variables|Default|SetSectionOpener (Variables|Default|GetFunkOpen_Cue))
      (Variables|Default|SetSectionBetween (Variables|Default|GetFunkBetween_Cue))
      (Variables|Default|SetSectionEnd (Variables|Default|GetFunkEnd))
      (switch int (Variables|/Game/Blueprints/GameMode.GameMode_C|GetGameMode _asgame_mode)
        (:0
          (Variables|Default|SetSection1 (Variables|Default|GetFunkRound1_OG_))
          (Variables|Default|SetSection2 (Variables|Default|GetFunkRound2))
          (Variables|Default|SetSection3 (Variables|Default|GetFunkRound3)))
        (:1
          (Variables|Default|SetSection1 (Variables|Default|GetFunkRound1))
          (Variables|Default|SetSection2 (Variables|Default|GetAIFunkRound2))
          (Variables|Default|SetSection3 (Variables|Default|GetAIFunkRound3)))))))

(fn ConstructionScript)

(fn NewFunction)
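; Player 1 input Blueprint for a rhythm mechanic that records snare hits on a sixteenth-note grid.
; Every Tick it looks up the first Beat actor and copies its current note (offset by one), note array and Player1Input flag.
; While that flag is true, pressing Z plays the Snare sound and marks the current sixteenth-note slot true in the Beat actor's array.
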(event EventTick
  (params (DeltaSeconds :type Float%20%28single-precision%29))
  (bind _outactors (Actor|GetAllActorsOfClass "/Game/Blueprints/Beat.Beat_C"))
  (Variables|Default|Set16thNote (+ (Variables|/Game/Blueprints/Beat.Beat_C|Get16thNote (Utilities|Array|Get(acopy) _outactors)) 1))
  (Variables|Default|Set16thNoteArray (Variables|/Game/Blueprints/Beat.Beat_C|Get16thNoteArray (Utilities|Array|Get(acopy) _outactors)))
  (Variables|Default|SetPlayer1Input (Variables|/Game/Blueprints/Beat.Beat_C|GetPlayer1Input (Utilities|Array|Get(acopy) _outactors))))

(event Input|KeyboardEvents|Z
  (params (Key :type Key%20Structure :default "None"))
  (:Pressed
    (if (Variables|Default|GetPlayer1Input)
      (Audio|Components|Audio|Play (Variables|Default|GetSnare) 0.0)
      (Utilities|Array|SetArrayElem (Variables|/Game/Blueprints/Beat.Beat_C|Get16thNoteArray (Utilities|Array|Get(acopy) (stale EventTick _outactors))) (- (Variables|Default|Get16thNote) 1) true))))

(fn ConstructionScript)
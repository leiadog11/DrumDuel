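; Main menu actor that hosts a widget and acts as a camera stop, linking to other menus through the LinkedMenus array.
; On BeginPlay it disables its collision and binds to its WB_Base widget's transition event, which passes a menu index.
; A valid index disables this actor's collision, enables the target menu's, and eases the player's view over to that menu with SetViewTargetWithBlend.
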(event Custom|TransitionTo
  (params (Main%20Menu :type BP%20Main%20Menu%20Object%20Reference))
  ;[1 1 1] Creation of TransitionToFunction Which Goes to a Camera
  (Collision|SetActorEnableCollision false)
  (Collision|SetActorEnableCollision Main%20Menu true)
  (Game|Player|SetViewTargetwithBlend (Game|GetPlayerController 0) Main%20Menu 2.0 "VTBlend_EaseInOut" 2.0 false))

(event Custom|OnTransitionBetweenMenus
  (params (MenuIndex :type Integer))
  (bind _linkedmenus (Variables|Default|GetLinkedMenus))
  ;[1 1 1] Cool Camera Trasitions by Going Through An Array of Cameras
  (if (Utilities|Array|IsValidIndex _linkedmenus MenuIndex)
    (CallFunction|Transitionto (Utilities|Array|Get(acopy) _linkedmenus MenuIndex))))

(event EventBeginPlay
  ;[1 1 1] Cool Camera Trasitions by Going Through An Array of Cameras
  (bind _aswb_base (Utilities|Casting|CastToWB_Base (UserInterface|GetUserWidgetObject (Variables|Default|GetWidget))))
  (EventDispatchers|BindEventtoTransitiontoLinkedMenu _aswb_base (delegate Custom|OnTransitionBetweenMenus))
  (Collision|SetActorEnableCollision false))

(event Collision|EventActorBeginOverlap
  (params (OtherActor :type Actor%20Object%20Reference)))

(event EventTick
  (params (DeltaSeconds :type Float%20%28single-precision%29)))

(fn ConstructionScript)
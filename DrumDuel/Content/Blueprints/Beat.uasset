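; Beat conductor for a three-phase drum duel, running turn order, announcer audio and on-screen prompts at a fixed 100 BPM.
; GoNext starts looping note-division timers and later resumes play between phases or returns to the main menu.
; Quarter-note counts hand off to a two-player or AI create/repeat turn cycle, chosen by GameMode, which resets note arrays.
; Phase ends change bar lengths and play interludes with placeholder crowd reactions.
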(event Custom|16th%20Notes
  ;[1 1 1] 16th Notes
  (Variables|Default|Set16thNote (+ (Variables|Default|Get16thNote) 1))
  (switch int (Variables|Default|GetPhase)
    (:1
      (if (== (Variables|Default|Get16thNote) 16)
        (Variables|Default|Set16thNote 0 :!label _label)))
    (:2
      (if (== (Variables|Default|Get16thNote) 32)
        (goto _label)))
    (:3
      (if (== (Variables|Default|Get16thNote) 64)
        (goto _label)))))

(event Custom|AITurnCycle
  (bind _snare (Variables|Default|GetSnare))
  (bind _visuals (Variables|Default|GetVisuals))
  (bind _visuals_2 (Variables|Default|GetVisuals))
  (bind _phase1notearray (Variables|Default|GetPhase1NoteArray))
  (bind _phase2notearray (Variables|Default|GetPhase2NoteArray))
  (bind _phase3notearray (Variables|Default|GetPhase3NoteArray))
  (bind _snare_2 (Variables|Default|GetSnare))
  ;[1 1 1] AI TURN CYCLE
  (if (and (not (Variables|Default|GetBetweenPhases)) (Variables|Default|GetSwitch))
    (bind _output_get (Variables|Default|SetHalfNote (+ (Variables|Default|GetHalfNote) 1)))
    (switch int _output_get
      (:1
        (bind _output_get_2 (Variables|Default|SetAITurnCycleInt (+ (Variables|Default|GetAITurnCycleInt) 1)))
        (if (== _output_get_2 3)
          (Variables|Default|SetAITurnCycleInt 1)
          (bind _output_get_3 (Variables|Default|SetCycleCount (+ (Variables|Default|GetCycleCount) 1)))
          (if (== _output_get_3 (Variables|Default|GetCycleCountAmount))
            (Variables|Default|SetBetweenPhases true)
            (Variables|Default|SetPhase (+ (Variables|Default|GetPhase) 1))
            (Variables|Default|SetCycleCount 0)
            ;[1 1 1] Phase Change
            (switch int (Variables|Default|GetPhase)
              (:2
                (Audio|Components|Audio|Play (Variables|Default|GetEnd1) 0.0) ; PHASE 1 SCORE
                (Rendering|Components|TextRender|SetText _visuals_2 (Variables|Text|GetEndOfPhase1))
                (Variables|Default|Set4thNoteAmount 8)
                (Variables|Default|SetCycleCountAmount 2)
                (Audio|Components|Audio|Play (Variables|Default|GetDrumDuelJazz_BetweenRoundInterlude_Cue) 0.0 :!label _label)
                ;[1 1 1] Crowd Cheers
                (Utilities|FlowControl|Delay 2.5)
                (Audio|Components|Audio|Play (Variables|Default|GetHear1Crowd) 0.0)
                (Utilities|FlowControl|Delay 2.0)
                (switch int (Variables|Default|GetPlayer1Crowd)
                  (:0
                    _)
                  (:1
                    (Audio|Components|Audio|Play (Variables|Default|GetSnare) 0.0))
                  (:2
                    (Audio|Components|Audio|Play (Variables|Default|GetSnare) 0.0))
                  (:3
                    (Audio|Components|Audio|Play (Variables|Default|GetSnare) 0.0))
                  (:4
                    (Audio|Components|Audio|Play (Variables|Default|GetSnare) 0.0))
                  (:5
                    (Audio|Components|Audio|Play _snare 0.0))
                  (:6
                    (Audio|Components|Audio|Play _snare 0.0)))
                (Utilities|FlowControl|Delay 4.0)
                (bind _asgame_mode (Utilities|Casting|CastToGameMode (Game|GetGameInstance)))
                (switch int (Variables|/Game/Blueprints/GameMode.GameMode_C|GetGameMode _asgame_mode)
                  (:0
                    (Audio|Components|Audio|Play (Variables|Default|GetHear2Crowd) 0.0)
                    (Utilities|FlowControl|Delay 2.0)
                    (switch int (Variables|Default|GetPlayer2Crowd)
                      (:0
                        _)
                      (:1
                        (Audio|Components|Audio|Play (Variables|Default|GetSnare) 0.0))
                      (:2
                        (Audio|Components|Audio|Play (Variables|Default|GetSnare) 0.0))
                      (:3
                        (Audio|Components|Audio|Play (Variables|Default|GetSnare) 0.0))
                      (:4
                        (Audio|Components|Audio|Play (Variables|Default|GetSnare) 0.0))
                      (:5
                        (Audio|Components|Audio|Play _snare_2 0.0))
                      (:6
                        (Audio|Components|Audio|Play _snare_2 0.0)))
                    (Utilities|FlowControl|Delay 4.0))
                  (:1
                    _))
                (Audio|Components|Audio|Play (Variables|Default|GetDrumToContinue) 0.0))
              (:3
                (Audio|Components|Audio|Play (Variables|Default|GetEnd2) 0.0) ; PHASE 2 SCORE
                (Rendering|Components|TextRender|SetText _visuals_2 (Variables|Text|GetEndOfPhase2))
                (Variables|Default|Set4thNoteAmount 16)
                (Variables|Default|SetCycleCountAmount 1)
                (goto _label))
              (:4
                (Audio|Components|Audio|Play (Variables|Default|GetEnd3) 0.0) ; PHASE 3 SCORE
                (Rendering|Components|TextRender|SetText _visuals_2 (Variables|Text|GetEndOfPhase3))
                (Audio|Components|Audio|Play (Variables|Default|GetDrumDuelJazz_Ending) 0.0)))
            (else
              (switch int (Variables|Default|GetAITurnCycleInt) :!label _label_2
                (:1
                  (Audio|Components|Audio|Play (Variables|Default|GetAICreate) 0.0)
                  (Rendering|Components|TextRender|SetText _visuals (Variables|Text|GetAICreateText))
                  (bind _returnvalue (Actor|GetActorOfClass "/Game/Blueprints/PlayerInput.PlayerInput_C"))
                  (Variables|/Game/Blueprints/PlayerInput.PlayerInput_C|SetNoteCounter _returnvalue 0.0)
                  (switch int (Variables|Default|GetPhase) ; RESET ARRAY OF NOTES
                    (:1
                      (for (_ _array_index) _phase1notearray
                        (Utilities|Array|SetArrayElem _phase1notearray _array_index false)
                        (bind _outactors (Actor|GetAllActorsOfClass "/Game/Blueprints/MusicHandler.MusicHandler_C"))
                        (Default|MusicCalled _outactors)))
                    (:2
                      (for (_ _array_index_2) _phase2notearray
                        (Utilities|Array|SetArrayElem _phase2notearray _array_index_2 false)
                        (bind _outactors_2 (Actor|GetAllActorsOfClass "/Game/Blueprints/MusicHandler.MusicHandler_C"))
                        (Default|MusicCalled _outactors_2)))
                    (:3
                      (for (_ _array_index_3) _phase3notearray
                        (Utilities|Array|SetArrayElem _phase3notearray _array_index_3 false)
                        (bind _outactors_3 (Actor|GetAllActorsOfClass "/Game/Blueprints/MusicHandler.MusicHandler_C"))
                        (Default|MusicCalled _outactors_3)))))
                (:2
                  (Audio|Components|Audio|Play (Variables|Default|GetP1Repeat) 0.0)
                  (Rendering|Components|TextRender|SetText _visuals (Variables|Text|GetP1RepeatText))))))
          (else
            (goto _label_2))))
      (:2
        (Audio|Components|Audio|Play (Variables|Default|GetGo) 0.0)
        (Rendering|Components|TextRender|SetText _visuals (Variables|Text|GetReadyGo))
        (Utilities|FlowControl|Delay (- (* (Variables|Default|GetSpeed) 2.0) 0.1))
        (Variables|Default|SetHalfNote 0)
        (Variables|Default|SetSwitch false)
        (Rendering|Components|TextRender|SetText _visuals (Variables|Text|GetBlank))))))

(event Custom|Quarter%20Notes
  ;[1 1 1] Quarter Notes
  (if (not (Variables|Default|GetSwitch))
    (Audio|Components|Audio|Play (Variables|Default|GetSmallBeat) 0.0)
    (bind _output_get (Variables|Default|SetQuarterNote (+ (Variables|Default|GetQuarterNote) 1)))
    (if (== _output_get (Variables|Default|Get4thNoteAmount))
      (Utilities|FlowControl|Delay (- (Variables|Default|GetSpeed) 0.1))
      (Variables|Default|SetSwitch true)
      (Variables|Default|SetQuarterNote 0))))

(event Custom|8th%20Notes
  ;[1 1 1] 8th Notes
)

(event Custom|GoNext
  (bind _speed (Variables|Default|GetSpeed))
  ;[1 1 1] Phase Change
  (if (Variables|Default|GetBetweenPhases)
    (Audio|Components|Audio|FadeOut (Variables|Default|GetDrumDuelJazz_BetweenRoundInterlude_Cue) 2.0 0.0 "Linear" :!class /Script/Engine.AudioComponent)
    (switch int (Variables|Default|GetPhase)
      (:0
        (Variables|Default|SetPhase 1)
        (Variables|Default|SetHalfNote 0)
        (Variables|Default|SetBetweenPhases false)
        ;[1 1 1] TIMERS
        (Audio|Components|Audio|Play (Variables|Default|GetCOMMENCE) 0.0) ; APPLAUSE AND START?
        (Audio|Components|Audio|FadeOut (Variables|Default|GetDrumDuelJazz_Opener_Cue) 4.0 0.0 "Linear" :!class /Script/Engine.AudioComponent)
        (Utilities|FlowControl|Delay 2.0)
        (Utilities|Time|SetTimerbyFunctionName 0 "Quarter Notes" _speed true false _speed)
        (bind _asgame_mode (Utilities|Casting|CastToGameMode (Game|GetGameInstance)))
        (switch int (Variables|/Game/Blueprints/GameMode.GameMode_C|GetGameMode _asgame_mode)
          (:0
            (Utilities|Time|SetTimerbyFunctionName 0 "TurnCycle" (* (Variables|Default|GetSpeed) 2.0) true))
          (:1
            (Utilities|Time|SetTimerbyFunctionName 0 "AITurnCycle" (* (Variables|Default|GetSpeed) 2.0) true)))
        (Utilities|Time|SetTimerbyFunctionName 0 "8th Notes" (/ (Variables|Default|GetSpeed) 2.0) true false 0.3)
        (Utilities|Time|SetTimerbyFunctionName 0 "16th Notes" (/ (Variables|Default|GetSpeed) 4.0) true false 0.45))
      (:2
        (Variables|Default|SetTurnCycleInt 0 :!label _label)
        (Variables|Default|SetAITurnCycleInt 0)
        (Variables|Default|SetHalfNote 0)
        (Rendering|Components|TextRender|SetText (Variables|Default|GetVisuals) (Variables|Text|GetBlank))
        (Variables|Default|SetBetweenPhases false))
      (:3
        (goto _label))
      (:4
        (Game|OpenLevel(byName) "Main_Menu")))))

(event Custom|TurnCycle
  (bind _snare (Variables|Default|GetSnare))
  (bind _visuals (Variables|Default|GetVisuals))
  (bind _visuals_2 (Variables|Default|GetVisuals))
  (bind _phase1notearray (Variables|Default|GetPhase1NoteArray))
  (bind _phase2notearray (Variables|Default|GetPhase2NoteArray))
  (bind _phase3notearray (Variables|Default|GetPhase3NoteArray))
  (bind _snare_2 (Variables|Default|GetSnare))
  ;[1 1 1] Turn Cycle
  (if (and (not (Variables|Default|GetBetweenPhases)) (Variables|Default|GetSwitch))
    (bind _output_get (Variables|Default|SetHalfNote (+ (Variables|Default|GetHalfNote) 1)))
    (switch int _output_get
      (:1
        (bind _output_get_2 (Variables|Default|SetTurnCycleInt (+ (Variables|Default|GetTurnCycleInt) 1)))
        (if (== _output_get_2 5)
          (Variables|Default|SetTurnCycleInt 1)
          (bind _output_get_3 (Variables|Default|SetCycleCount (+ (Variables|Default|GetCycleCount) 1)))
          (if (== _output_get_3 (Variables|Default|GetCycleCountAmount))
            (Variables|Default|SetBetweenPhases true)
            (Variables|Default|SetPhase (+ (Variables|Default|GetPhase) 1))
            (Variables|Default|SetCycleCount 0)
            ;[1 1 1] Phase Change
            (switch int (Variables|Default|GetPhase)
              (:2
                (Audio|Components|Audio|Play (Variables|Default|GetEnd1) 0.0) ; PHASE 1 SCORE
                (Rendering|Components|TextRender|SetText _visuals (Variables|Text|GetEndOfPhase1))
                (Variables|Default|Set4thNoteAmount 8)
                (Variables|Default|SetCycleCountAmount 2)
                (Audio|Components|Audio|Play (Variables|Default|GetDrumDuelJazz_BetweenRoundInterlude_Cue) 0.0 :!label _label)
                ;[1 1 1] Crowd Cheers
                (Utilities|FlowControl|Delay 2.5)
                (Audio|Components|Audio|Play (Variables|Default|GetHear1Crowd) 0.0)
                (Utilities|FlowControl|Delay 2.0)
                (switch int (Variables|Default|GetPlayer1Crowd)
                  (:0
                    _)
                  (:1
                    (Audio|Components|Audio|Play (Variables|Default|GetSnare) 0.0))
                  (:2
                    (Audio|Components|Audio|Play (Variables|Default|GetSnare) 0.0))
                  (:3
                    (Audio|Components|Audio|Play (Variables|Default|GetSnare) 0.0))
                  (:4
                    (Audio|Components|Audio|Play (Variables|Default|GetSnare) 0.0))
                  (:5
                    (Audio|Components|Audio|Play _snare 0.0))
                  (:6
                    (Audio|Components|Audio|Play _snare 0.0)))
                (Utilities|FlowControl|Delay 4.0)
                (bind _asgame_mode (Utilities|Casting|CastToGameMode (Game|GetGameInstance)))
                (switch int (Variables|/Game/Blueprints/GameMode.GameMode_C|GetGameMode _asgame_mode)
                  (:0
                    (Audio|Components|Audio|Play (Variables|Default|GetHear2Crowd) 0.0)
                    (Utilities|FlowControl|Delay 2.0)
                    (switch int (Variables|Default|GetPlayer2Crowd)
                      (:0
                        _)
                      (:1
                        (Audio|Components|Audio|Play (Variables|Default|GetSnare) 0.0))
                      (:2
                        (Audio|Components|Audio|Play (Variables|Default|GetSnare) 0.0))
                      (:3
                        (Audio|Components|Audio|Play (Variables|Default|GetSnare) 0.0))
                      (:4
                        (Audio|Components|Audio|Play (Variables|Default|GetSnare) 0.0))
                      (:5
                        (Audio|Components|Audio|Play _snare_2 0.0))
                      (:6
                        (Audio|Components|Audio|Play _snare_2 0.0)))
                    (Utilities|FlowControl|Delay 4.0))
                  (:1
                    _))
                (Audio|Components|Audio|Play (Variables|Default|GetDrumToContinue) 0.0))
              (:3
                (Audio|Components|Audio|Play (Variables|Default|GetEnd2) 0.0) ; PHASE 2 SCORE
                (Rendering|Components|TextRender|SetText _visuals (Variables|Text|GetEndOfPhase2))
                (Variables|Default|Set4thNoteAmount 16)
                (Variables|Default|SetCycleCountAmount 1)
                (goto _label))
              (:4
                (Audio|Components|Audio|Play (Variables|Default|GetEnd3) 0.0) ; PHASE 3 SCORE
                (Rendering|Components|TextRender|SetText _visuals (Variables|Text|GetEndOfPhase3))
                (Audio|Components|Audio|Play (Variables|Default|GetDrumDuelJazz_Ending) 0.0)))
            (else
              (switch int (Variables|Default|GetTurnCycleInt) :!label _label_2
                (:1
                  (Audio|Components|Audio|Play (Variables|Default|GetP1Create) 0.0)
                  (Rendering|Components|TextRender|SetText _visuals_2 (Variables|Text|GetP1CreateText))
                  (bind _returnvalue (Actor|GetActorOfClass "/Game/Blueprints/PlayerInput.PlayerInput_C" :!label _label_3))
                  (Variables|/Game/Blueprints/PlayerInput.PlayerInput_C|SetNoteCounter _returnvalue 0.0)
                  (switch int (Variables|Default|GetPhase) ; RESET ARRAY OF NOTES
                    (:1
                      (for (_ _array_index) _phase1notearray
                        (Utilities|Array|SetArrayElem _phase1notearray _array_index false)
                        (bind _outactors (Actor|GetAllActorsOfClass "/Game/Blueprints/MusicHandler.MusicHandler_C"))
                        (Default|MusicCalled _outactors)))
                    (:2
                      (for (_ _array_index_2) _phase2notearray
                        (Utilities|Array|SetArrayElem _phase2notearray _array_index_2 false)
                        (bind _outactors_2 (Actor|GetAllActorsOfClass "/Game/Blueprints/MusicHandler.MusicHandler_C"))
                        (Default|MusicCalled _outactors_2)))
                    (:3
                      (for (_ _array_index_3) _phase3notearray
                        (Utilities|Array|SetArrayElem _phase3notearray _array_index_3 false)
                        (bind _outactors_3 (Actor|GetAllActorsOfClass "/Game/Blueprints/MusicHandler.MusicHandler_C"))
                        (Default|MusicCalled _outactors_3)))))
                (:2
                  (Audio|Components|Audio|Play (Variables|Default|GetP2Repeat) 0.0)
                  (Rendering|Components|TextRender|SetText _visuals_2 (Variables|Text|GetP2RepeatText)))
                (:3
                  (Audio|Components|Audio|Play (Variables|Default|GetP2Create) 0.0)
                  (Rendering|Components|TextRender|SetText _visuals_2 (Variables|Text|GetP2CreateText))
                  (goto _label_3))
                (:4
                  (Audio|Components|Audio|Play (Variables|Default|GetP1Repeat) 0.0)
                  (Rendering|Components|TextRender|SetText _visuals_2 (Variables|Text|GetP1RepeatText))))))
          (else
            (goto _label_2))))
      (:2
        (Audio|Components|Audio|Play (Variables|Default|GetGo) 0.0)
        (Rendering|Components|TextRender|SetText _visuals_2 (Variables|Text|GetReadyGo))
        (Utilities|FlowControl|Delay (- (* (Variables|Default|GetSpeed) 2.0) 0.1))
        (Variables|Default|SetHalfNote 0)
        (Variables|Default|SetSwitch false)
        (Rendering|Components|TextRender|SetText _visuals_2 (Variables|Text|GetBlank))))))

(event EventBeginPlay
  ;[1 1 1] SET BPM AND NOTE SPEED
  (Variables|Default|SetBPM 1e+02) ; SET BPM FROM SETTINGS! (100 BY DEFAULT)
  (Variables|Default|SetSpeed (/ 6e+01 (Variables|Default|GetBPM))) ; SETS SPEED FOR QUARTER NOTES
  ;[1 1 1] TUTORIAL
  (Audio|Components|Audio|Play (Variables|Default|GetDrumDuelJazz_Opener_Cue) 0.0)
  (Audio|Components|Audio|Play (Variables|Default|GetWelcome) 0.0))

(fn ConstructionScript)